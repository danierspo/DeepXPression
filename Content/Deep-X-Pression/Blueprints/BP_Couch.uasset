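; Interactable couch and dialogue participant where Emil can hold a group conversation or relax alone, affecting his mood.
; Overlap shows a prompt widget and enables input; interacting starts dialogue depending on whether the clock reads hour 12.
; Custom events hide teleporting four coworkers and advancing two linked clocks behind camera fades.
; The group talk sets mood to 100, while solo relaxing adds mood proportional to minutes remaining in the hour.
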(event `self.ReceiveBeginPlay`
  ;[1 1 1] BeginPlay: obtain reference to BP_Emil player character
  (bind _asbp_emil (cast `/Game/Deep-X-Pression/Blueprints/BP_Emil` (`Controller.K2_GetPawn` (`GameplayStatics.GetPlayerController` 0))))
  (set `self.Emil` _asbp_emil))

(event `InputAction|Interact`
  (params (Key :type "Key Structure"))
  ;[1 1 1] Press E to interact with the couch
  (:`Pressed`
    (if (`self.CanInteract`)
      (`self.OnInteract`)
      (else
        (`/Game/Deep-X-Pression/Blueprints/BP_Emil.StartDialogue` (`self.Emil`) "/Game/Deep-X-Pression/Dialogues/Dlg_Emil_CannotInteract.Dlg_Emil_CannotInteract")))))

(event `self.ReceiveActorBeginOverlap`
  (params (OtherActor :type "Actor Object Reference"))
  ;[1 1 1] Couch overlapping with character
  (cast `Character` OtherActor)
  (bind _returnvalue (`|CreateWidget` "/Game/Deep-X-Pression/UI/InteractPrompts/IP_Couch.IP_Couch_C"))
  (`UserWidget.AddToViewport` _returnvalue 0)
  (`self.EnableInput` (`GameplayStatics.GetPlayerController` 0)))

(event `self.ReceiveActorEndOverlap`
  (params (OtherActor :type "Actor Object Reference"))
  ;[1 1 1] Couch overlapping with character
  (cast `Character` OtherActor)
  (`Widget.RemoveFromParent` (stale `self.ReceiveActorBeginOverlap` _returnvalue))
  (`self.DisableInput` (`GameplayStatics.GetPlayerController` 0)))

(event `self.OnInteract`
  (bind _emil (`self.Emil`))
  ;[1 1 1] Interactable's OnInteract method implementation
  (if (== (`/Game/Deep-X-Pression/Blueprints/BP_AnalogClock.Hours` (`self.Clock`)) 12)
    (`/Game/Deep-X-Pression/Blueprints/BP_Emil.StartDialogue` _emil "/Game/Deep-X-Pression/Dialogues/Dlg_EmilCouch.Dlg_EmilCouch")
    (else
      (`/Game/Deep-X-Pression/Blueprints/BP_Emil.StartDialogue` _emil "/Game/Deep-X-Pression/Dialogues/Dlg_EmilCouch_Not12.Dlg_EmilCouch_Not12"))))

(event `ImportantDialogue_Start`
  (bind _returnvalue (`GameplayStatics.GetPlayerCameraManager` 0))
  (bind _emil (`self.Emil`))
  ;[1 1 1] Harry, Jennifer, Kevin and Laura on the couch, then starts the important dialogue
  (`PlayerCameraManager.StartCameraFade` _returnvalue 0.0 1.0 1.0 (struct :`A` 1.0) false true)
  (`KismetSystemLibrary.Delay` 2.0)
  (`self.K2_SetActorLocationAndRotation` :`self` (`self.Harry`) :`NewLocation` (2804.0 2089.0 8.0))
  (`self.K2_SetActorLocationAndRotation` (`self.Jennifer`) (2873.0 2140.0 14.0) (struct :`Yaw` 90.0) false false)
  (`self.K2_SetActorLocationAndRotation` (`self.Kevin`) (2906.0 2200.0 8.0) (struct :`Yaw` 90.0) false false)
  (`self.K2_SetActorLocationAndRotation` (`self.Laura`) (2870.0 2280.0 9.0) (struct :`Yaw` 90.0) false false)
  (`PlayerCameraManager.StartCameraFade` _returnvalue 1.0 0.0 1.0 (struct :`A` 1.0) false true)
  (`/Game/Deep-X-Pression/Blueprints/BP_Emil.StartDialogue` _emil "/Game/Deep-X-Pression/Dialogues/Dlg_ImportantDialogue.Dlg_ImportantDialogue")
  (set `/Game/Deep-X-Pression/Blueprints/BP_Emil.Mood` 100.0 _emil))

(event `ImportantDialogue_End`
  (bind _returnvalue (`GameplayStatics.GetPlayerCameraManager` 0))
  (bind _clock (`self.Clock`))
  (bind _otherclock (`/Game/Deep-X-Pression/Blueprints/BP_AnalogClock.OtherClock` _clock))
  ;[1 1 1] Harry, Jennifer, Kevin and Laura return to their workspace, then the player control returns to Emil
  (`PlayerCameraManager.StartCameraFade` _returnvalue 0.0 1.0 1.0 (struct :`A` 1.0) false true)
  (`KismetSystemLibrary.Delay` 2.0)
  (set `/Game/Deep-X-Pression/Blueprints/BP_AnalogClock.CouchAdvance` true _clock)
  (`/Game/Deep-X-Pression/Blueprints/BP_AnalogClock.OnInteract` _clock)
  (set `/Game/Deep-X-Pression/Blueprints/BP_AnalogClock.CouchAdvance` true _otherclock)
  (`/Game/Deep-X-Pression/Blueprints/BP_AnalogClock.OnInteract` _otherclock)
  (`KismetSystemLibrary.Delay` 1.0)
  (`self.K2_SetActorLocationAndRotation` :`self` (`self.Harry`) :`NewLocation` (1080.0 1570.0 3.0))
  (`self.K2_SetActorLocationAndRotation` :`self` (`self.Jennifer`) :`NewLocation` (1932.0 1560.0 7.0))
  (`self.K2_SetActorLocationAndRotation` :`self` (`self.Kevin`) :`NewLocation` (1080.0 1175.0 5.0))
  (`self.K2_SetActorLocationAndRotation` :`self` (`self.Laura`) :`NewLocation` (1932.0 1185.0 5.0))
  (`PlayerCameraManager.StartCameraFade` _returnvalue 1.0 0.0 1.0 (struct :`A` 1.0) false true))

(event `RelaxByYourself`
  (bind _returnvalue (`GameplayStatics.GetPlayerCameraManager` 0))
  (bind _clock (`self.Clock`))
  (bind _otherclock (`/Game/Deep-X-Pression/Blueprints/BP_AnalogClock.OtherClock` _clock))
  ;[1 1 1] Time elapses to 13:00 while Emil spends his time alone on the couch
  (`PlayerCameraManager.StartCameraFade` _returnvalue 0.0 1.0 1.0 (struct :`A` 1.0) false true)
  (`KismetSystemLibrary.Delay` 2.0)
  (set `/Game/Deep-X-Pression/Blueprints/BP_AnalogClock.CouchAdvance` true _clock)
  (`/Game/Deep-X-Pression/Blueprints/BP_AnalogClock.OnInteract` _clock)
  (set `/Game/Deep-X-Pression/Blueprints/BP_AnalogClock.CouchAdvance` true _otherclock)
  (`/Game/Deep-X-Pression/Blueprints/BP_AnalogClock.OnInteract` _otherclock)
  (`KismetSystemLibrary.Delay` 1.0)
  (bind _newmood (`/Game/Deep-X-Pression/Blueprints/BP_Emil.AddToMood` (`self.Emil`) (* (`KismetMathLibrary.Conv_IntToDouble` (- 61 (`/Game/Deep-X-Pression/Blueprints/BP_AnalogClock.Minutes` (`self.Clock`)))) 0.25)))
  (`PlayerCameraManager.StartCameraFade` _returnvalue 1.0 0.0 1.0 (struct :`A` 1.0) false true)
  (`KismetSystemLibrary.PrintText` (`|FormatText` "Ti sei rilassato. Ora, l'umore di Emil è {Mood}." _newmood)))

(fn `CheckCondition`
  (params (Context :type "DlgContext Object Reference") (ConditionName :type Name))
  (returns (ReturnValue :type Boolean))
  (return false))

(fn `GetBoolValue`
  (params (ValueName :type Name))
  (returns (ReturnValue :type Boolean))
  (return false))

(fn `GetFloatValue`
  (params (ValueName :type Name))
  (returns (ReturnValue :type "Float (single-precision)"))
  (return 0.0))

(fn `GetIntValue`
  (params (ValueName :type Name))
  (returns (ReturnValue :type Integer))
  (return 0))

(fn `GetNameValue`
  (params (ValueName :type Name))
  (returns (ReturnValue :type Name))
  (return "None"))

(fn `GetParticipantDisplayName`
  (params (ActiveSpeaker :type Name))
  (returns (ReturnValue :type Text))
  (return (`self.DisplayName`)))

(fn `GetParticipantGender`
  (returns (ReturnValue :type "ETextGender Enum"))
  (return "Masculine"))

(fn `GetParticipantIcon`
  (params (ActiveSpeaker :type Name) (ActiveSpeakerState :type Name))
  (returns (ReturnValue :type "Texture2D Object Reference"))
  (return "/Game/Deep-X-Pression/Assets/CouchAndTV.CouchAndTV"))

(fn `GetParticipantName`
  (returns (ReturnValue :type Name))
  (return "Couch"))

(fn `ModifyBoolValue`
  (params (ValueName :type Name) (bNewValue :type Boolean))
  (returns (ReturnValue :type Boolean))
  (return false))

(fn `ModifyFloatValue`
  (params (ValueName :type Name) (bDelta :type Boolean) (Value :type "Float (single-precision)"))
  (returns (ReturnValue :type Boolean))
  (return false))

(fn `ModifyIntValue`
  (params (ValueName :type Name) (bDelta :type Boolean) (Value :type Integer))
  (returns (ReturnValue :type Boolean))
  (return false))

(fn `ModifyNameValue`
  (params (ValueName :type Name) (NameValue :type Name))
  (returns (ReturnValue :type Boolean))
  (return false))

(fn `OnDialogueEvent`
  (params (Context :type "DlgContext Object Reference") (EventName :type Name))
  (returns (ReturnValue :type Boolean))
  (return false))

(fn `UserConstructionScript`)