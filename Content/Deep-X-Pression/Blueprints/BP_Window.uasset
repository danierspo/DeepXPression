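; BP_Window is an interactable window that starts dialogues with the player character, Emil.
; Overlapping characters show a prompt widget and enable input, so Interact plays the window dialogue or a cannot-interact one, depending on CanInteract.
; Per-character toggle functions write the inverse of this window's important-dialogue flag to every BP_Window.
; It implements the dialogue participant interface, returning its name, display name and icon, with other methods mostly stubbed.
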(event `self.ReceiveBeginPlay`
  ;[1 1 1] BeginPlay: obtain reference to BP_Emil player character
  (bind _asbp_emil (cast `/Game/Deep-X-Pression/Blueprints/BP_Emil` (`Controller.K2_GetPawn` (`GameplayStatics.GetPlayerController` 0))))
  (set `self.Emil` _asbp_emil))

(event `InputAction|Interact`
  (params (Key :type "Key Structure"))
  ;[1 1 1] Press E to interact with the window
  (:`Pressed`
    (if (`self.CanInteract`)
      (`self.OnInteract`)
      (else
        (`/Game/Deep-X-Pression/Blueprints/BP_Emil.StartDialogue` (`self.Emil`) "/Game/Deep-X-Pression/Dialogues/Dlg_Emil_CannotInteract.Dlg_Emil_CannotInteract")))))

(event `self.ReceiveActorBeginOverlap`
  (params (OtherActor :type "Actor Object Reference"))
  ;[1 1 1] Window overlapping with player character
  (cast `Character` OtherActor)
  (bind _returnvalue (`|CreateWidget` "/Game/Deep-X-Pression/UI/InteractPrompts/IP_Window.IP_Window_C"))
  (`UserWidget.AddToViewport` _returnvalue 0)
  (`self.EnableInput` (`GameplayStatics.GetPlayerController` 0)))

(event `self.ReceiveActorEndOverlap`
  (params (OtherActor :type "Actor Object Reference"))
  ;[1 1 1] Window overlapping with player character
  (cast `Character` OtherActor)
  (`Widget.RemoveFromParent` (stale `self.ReceiveActorBeginOverlap` _returnvalue))
  (`self.DisableInput` (`GameplayStatics.GetPlayerController` 0)))

(event `self.OnInteract`
  ;[1 1 1] Interactable's OnInteract method implementation
  (`/Game/Deep-X-Pression/Blueprints/BP_Emil.StartDialogue` (`self.Emil`) "/Game/Deep-X-Pression/Dialogues/Dlg_EmilWindow.Dlg_EmilWindow"))

(fn `CheckCondition`
  (params (Context :type "DlgContext Object Reference") (ConditionName :type Name))
  (returns (ReturnValue :type Boolean))
  (return false))

(fn `GetBoolValue`
  (params (ValueName :type Name))
  (returns (ReturnValue :type Boolean))
  (return false))

(fn `GetFloatValue`
  (params (ValueName :type Name))
  (returns (ReturnValue :type "Float (single-precision)"))
  (return 0.0))

(fn `GetIntValue`
  (params (ValueName :type Name))
  (returns (ReturnValue :type Integer))
  (return 0))

(fn `GetNameValue`
  (params (ValueName :type Name))
  (returns (ReturnValue :type Name))
  (return "None"))

(fn `GetParticipantDisplayName`
  (params (ActiveSpeaker :type Name))
  (returns (ReturnValue :type Text))
  (return (`self.DlgDisplayName`)))

(fn `GetParticipantGender`
  (returns (ReturnValue :type "ETextGender Enum"))
  (return "Masculine"))

(fn `GetParticipantIcon`
  (params (ActiveSpeaker :type Name) (ActiveSpeakerState :type Name))
  (returns (ReturnValue :type "Texture2D Object Reference"))
  (return (`self.DlgIcon`)))

(fn `GetParticipantName`
  (returns (ReturnValue :type Name))
  (return (`self.DlgName`)))

(fn `ModifyBoolValue`
  (params (ValueName :type Name) (bNewValue :type Boolean))
  (returns (ReturnValue :type Boolean))
  (return false))

(fn `ModifyFloatValue`
  (params (ValueName :type Name) (bDelta :type Boolean) (Value :type "Float (single-precision)"))
  (returns (ReturnValue :type Boolean))
  (return false))

(fn `ModifyIntValue`
  (params (ValueName :type Name) (bDelta :type Boolean) (Value :type Integer))
  (returns (ReturnValue :type Boolean))
  (return false))

(fn `ModifyNameValue`
  (params (ValueName :type Name) (NameValue :type Name))
  (returns (ReturnValue :type Boolean))
  (return false))

(fn `OnDialogueEvent`
  (params (Context :type "DlgContext Object Reference") (EventName :type Name))
  (returns (ReturnValue :type Boolean))
  (return false))

(fn `ToggleImportantDialogueHarry`
  (bind _outactors (`GameplayStatics.GetAllActorsOfClass` "BP_Window_C"))
  (for _array_element _outactors
    (set `/Game/Deep-X-Pression/Blueprints/BP_Window.ImportantDialogue_Harry` (not (`self.ImportantDialogue_Harry`)) _array_element)))

(fn `ToggleImportantDialogueJennifer`
  (bind _outactors (`GameplayStatics.GetAllActorsOfClass` "BP_Window_C"))
  (for _array_element _outactors
    (set `/Game/Deep-X-Pression/Blueprints/BP_Window.ImportantDialogue_Jennifer` (not (`self.ImportantDialogue_Jennifer`)) _array_element)))

(fn `ToggleImportantDialogueKevin`
  (bind _outactors (`GameplayStatics.GetAllActorsOfClass` "BP_Window_C"))
  (for _array_element _outactors
    (set `/Game/Deep-X-Pression/Blueprints/BP_Window.ImportantDialogue_Kevin` (not (`self.ImportantDialogue_Kevin`)) _array_element)))

(fn `ToggleImportantDialogueLaura`
  (bind _outactors (`GameplayStatics.GetAllActorsOfClass` "BP_Window_C"))
  (for _array_element _outactors
    (set `/Game/Deep-X-Pression/Blueprints/BP_Window.ImportantDialogue_Laura` (not (`self.ImportantDialogue_Laura`)) _array_element)))

(fn `UserConstructionScript`)