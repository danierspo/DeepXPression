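; Interactive analog clock that runs the in-game workday, rotating its hands on Tick and opening the exit door at 17:00.
; A looping AdvanceTime timer counts minutes and changes rate for desk, couch and fast-forward modes.
; Interacting spends Emil's mood to skip an hour on this and a linked clock.
; On the controlling clock, desk time restores mood, completes coworkers' tasks with dialogue and re-enables their conversations.
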(event `self.ReceiveBeginPlay`
  ;[1 1 1] BeginPlay: set timer at game start, which manages in-game clock (AdvanceTime custom event)
  (bind _asbp_emil (cast `/Game/Deep-X-Pression/Blueprints/BP_Emil` (`Controller.K2_GetPawn` (`GameplayStatics.GetPlayerController` 0))))
  (set `self.Emil` _asbp_emil)
  (bind _returnvalue (`KismetSystemLibrary.K2_SetTimerDelegate` (delegate `AdvanceTime`) (`self.SecondsDelay`) true))
  (bind _output_get (set `self.Timer` _returnvalue)))

(event `AdvanceTime`
  (bind _emildesk (`self.EmilDesk`))
  (bind _emil (`self.Emil`))
  (bind _deskadvance_timeelasped (`self.DeskAdvance_TimeElasped`))
  ;[1 1 1] BeginPlay: set timer at game start, which manages in-game clock (AdvanceTime custom event)
  (if (`self.CanInteract`)
    (if (and (`self.GameControlClock`) (`self.DeskAdvance`))
      (`/Engine/EditorBlueprintResources/StandardMacros.IncrementInt` _deskadvance_timeelasped
        (:`  `
          (if (== _deskadvance_timeelasped 60)
            (set `/Game/Deep-X-Pression/Other/BP_SecondaryCharacter.CanConverse` true (`self.Harry`))
            (set `/Game/Deep-X-Pression/Other/BP_SecondaryCharacter.CanConverse` true (`self.Jennifer`))
            (set `/Game/Deep-X-Pression/Other/BP_SecondaryCharacter.CanConverse` true (`self.Kevin`))
            (set `/Game/Deep-X-Pression/Other/BP_SecondaryCharacter.CanConverse` true (`self.Laura`))
            (set `self.DeskAdvance_TimeElasped` 0)
            (`/Game/Deep-X-Pression/Blueprints/BP_Emil.AddToMood` (`self.Emil`) 5.0)
            (if (`/Game/Deep-X-Pression/Blueprints/BP_EmilDesk.WorkToDo_Harry` _emildesk)
              (set `/Game/Deep-X-Pression/Blueprints/BP_EmilDesk.WorkToDo_Harry` false _emildesk)
              (set `/Game/Deep-X-Pression/Other/BP_SecondaryCharacter.WorkToDo_Completed` true (`self.Harry`))
              (`/Game/Deep-X-Pression/Blueprints/BP_Emil.StartDialogue` _emil "/Game/Deep-X-Pression/Dialogues/Dlg_WorkCompletedForHarry.Dlg_WorkCompletedForHarry")
              (elif (`/Game/Deep-X-Pression/Blueprints/BP_EmilDesk.WorkToDo_Jennifer` _emildesk)
                (set `/Game/Deep-X-Pression/Blueprints/BP_EmilDesk.WorkToDo_Jennifer` false _emildesk)
                (set `/Game/Deep-X-Pression/Other/BP_SecondaryCharacter.WorkToDo_Completed` true (`self.Jennifer`))
                (`/Game/Deep-X-Pression/Blueprints/BP_Emil.StartDialogue` _emil "/Game/Deep-X-Pression/Dialogues/Dlg_WorkCompletedForJennifer.Dlg_WorkCompletedForJennifer")
                (elif (`/Game/Deep-X-Pression/Blueprints/BP_EmilDesk.WorkToDo_Kevin` _emildesk)
                  (set `/Game/Deep-X-Pression/Blueprints/BP_EmilDesk.WorkToDo_Kevin` false _emildesk)
                  (set `/Game/Deep-X-Pression/Other/BP_SecondaryCharacter.WorkToDo_Completed` true (`self.Kevin`))
                  (`/Game/Deep-X-Pression/Blueprints/BP_Emil.StartDialogue` _emil "/Game/Deep-X-Pression/Dialogues/Dlg_WorkCompletedForKevin.Dlg_WorkCompletedForKevin")
                  (elif (`/Game/Deep-X-Pression/Blueprints/BP_EmilDesk.WorkToDo_Laura` _emildesk)
                    (set `/Game/Deep-X-Pression/Blueprints/BP_EmilDesk.WorkToDo_Laura` false _emildesk)
                    (set `/Game/Deep-X-Pression/Other/BP_SecondaryCharacter.WorkToDo_Completed` true (`self.Laura`))
                    (`/Game/Deep-X-Pression/Blueprints/BP_Emil.StartDialogue` _emil "/Game/Deep-X-Pression/Dialogues/Dlg_WorkCompletedForLaura.Dlg_WorkCompletedForLaura")))))
            (else
              (bind _result (`/Engine/EditorBlueprintResources/StandardMacros.IncrementInt` (`self.Minutes`) :!label _label)
                (:`  `
                  (set `self.Minutes` _result)
                  (if (== (`self.Minutes`) 60)
                    (bind _result_2 (`/Engine/EditorBlueprintResources/StandardMacros.IncrementInt` (`self.Hours`))
                      (:`  `
                        (set `self.Minutes` 0)
                        (if (== _result_2 17)
                          (set `self.CanInteract` false)
                          (set `/Game/Deep-X-Pression/Blueprints/BP_EmilDesk.CanInteract` false (`self.EmilDesk`))
                          (set `/Game/Deep-X-Pression/Blueprints/BP_ExitDoor.CanLeave` true (`self.ExitDoor`))
                          (`KismetSystemLibrary.K2_PauseTimerHandle` (stale `self.ReceiveBeginPlay` _output_get))))))))))))
      (else
        (goto _label)))
    (elif (`self.DeskAdvance`)
      (bind _output_get (set `self.SecondsDelay` 1.0))
      (`KismetSystemLibrary.K2_ClearAndInvalidateTimerHandle` (`self.Timer`))
      (bind _returnvalue (`KismetSystemLibrary.K2_SetTimerDelegate` (delegate `AdvanceTime`) _output_get true))
      (set `self.Timer` _returnvalue)
      (set `self.CanInteract` true)
      (else
        (if (`self.CouchAdvance`)
          (if (and (== (`self.Hours`) 13) (== (`self.Minutes`) 0))
            (set `self.CouchAdvance` false)
            (else
              (goto _label)))
          (elif (or (== (`self.temp`) (`self.Minutes`)) (== (`self.Hours`) 17))
            (`KismetSystemLibrary.PrintString` "Orologio nuovamente in funzione regolare")
            (else
              (goto _label))))
        (bind _output_get_2 (set `self.SecondsDelay` 10.0))
        (`KismetSystemLibrary.K2_ClearAndInvalidateTimerHandle` (`self.Timer`))
        (bind _returnvalue_2 (`KismetSystemLibrary.K2_SetTimerDelegate` (delegate `AdvanceTime`) _output_get_2 true))
        (set `self.Timer` _returnvalue_2)
        (set `self.CanInteract` true)))))

(event `self.ReceiveTick`
  (params (DeltaSeconds :type "Float (single-precision)"))
  (bind _minutes (`self.Minutes`))
  ;[1 1 1] Event tick to modify the clock graphycally based on current in-game time
  (`SceneComponent.K2_SetRelativeRotation` (`self.Minutes_Hand_Base`) (`KismetMathLibrary.MakeRotator` 0.0 0.0 (* (`self.SmoothMinutes` _minutes) 6.0)) false false)
  (`SceneComponent.K2_SetRelativeRotation` (`self.Hours_Hand_Base`) (`KismetMathLibrary.MakeRotator` 0.0 0.0 (`KismetMathLibrary.Conv_IntToDouble` (+ (* (`self.Hours`) 30) (/ _minutes 2)))) false false))

(event `InputAction|Interact`
  (params (Key :type "Key Structure"))
  (bind _emil (`self.Emil`))
  (bind _harry (`self.Harry`))
  (bind _jennifer (`self.Jennifer`))
  (bind _kevin (`self.Kevin`))
  (bind _laura (`self.Laura`))
  ;[1 1 1] Press E to fast forward time by one hour
  (:`Pressed`
    (if (`self.CanInteract`)
      (if (>= (`/Game/Deep-X-Pression/Blueprints/BP_Emil.Mood` _emil) 5.0)
        (`self.OnInteract`)
        (`self.OnInteract` (`self.OtherClock`))
        (bind _newmood (`/Game/Deep-X-Pression/Blueprints/BP_Emil.AddToMood` (`self.Emil`) -5.0))
        (`KismetSystemLibrary.Delay` 2.0)
        (if (== (`self.Hours`) 17)
          (set `/Game/Deep-X-Pression/Other/BP_SecondaryCharacter.CanConverse` false _harry)
          (set `/Game/Deep-X-Pression/Other/BP_SecondaryCharacter.CanConverse` false _jennifer)
          (set `/Game/Deep-X-Pression/Other/BP_SecondaryCharacter.CanConverse` false _kevin)
          (set `/Game/Deep-X-Pression/Other/BP_SecondaryCharacter.CanConverse` false _laura)
          (set `self.CanInteract` false)
          (set `/Game/Deep-X-Pression/Blueprints/BP_EmilDesk.CanInteract` false (`self.EmilDesk`))
          (set `/Game/Deep-X-Pression/Blueprints/BP_ExitDoor.CanLeave` true (`self.ExitDoor`))
          (elif (> _newmood 0.0)
            (set `/Game/Deep-X-Pression/Other/BP_SecondaryCharacter.CanConverse` true _harry)
            (set `/Game/Deep-X-Pression/Other/BP_SecondaryCharacter.CanConverse` true _jennifer)
            (set `/Game/Deep-X-Pression/Other/BP_SecondaryCharacter.CanConverse` true _kevin)
            (set `/Game/Deep-X-Pression/Other/BP_SecondaryCharacter.CanConverse` true _laura)))
        (else
          (`/Game/Deep-X-Pression/Blueprints/BP_Emil.StartDialogue` _emil "/Game/Deep-X-Pression/Dialogues/Dlg_Clock_CannotFastForward.Dlg_Clock_CannotFastForward")))
      (else
        (`KismetSystemLibrary.PrintString` "Al momento non puoi avanzare di un'ora.")))))

(event `self.ReceiveActorBeginOverlap`
  (params (OtherActor :type "Actor Object Reference"))
  ;[1 1 1] Clock overlapping with character
  (cast `Character` OtherActor)
  (bind _returnvalue (`|CreateWidget` "/Game/Deep-X-Pression/UI/InteractPrompts/IP_Clock.IP_Clock_C"))
  (`UserWidget.AddToViewport` _returnvalue 0)
  (`self.EnableInput` (`GameplayStatics.GetPlayerController` 0)))

(event `self.ReceiveActorEndOverlap`
  (params (OtherActor :type "Actor Object Reference"))
  ;[1 1 1] Clock overlapping with character
  (cast `Character` OtherActor)
  (`Widget.RemoveFromParent` (stale `self.ReceiveActorBeginOverlap` _returnvalue))
  (`self.DisableInput` (`GameplayStatics.GetPlayerController` 0)))

(event `self.OnInteract`
  (bind _minutes (`self.Minutes`))
  ;[1 1 1] Interactable's OnInteract method implementation
  (bind _output_get (set `self.SecondsDelay` 0.01))
  (`KismetSystemLibrary.K2_ClearAndInvalidateTimerHandle` (`self.Timer`))
  (bind _returnvalue (`KismetSystemLibrary.K2_SetTimerDelegate` (delegate `AdvanceTime`) _output_get true))
  (set `self.Timer` _returnvalue)
  (set `self.CanInteract` false)
  (set `self.temp` _minutes)
  (`/Engine/EditorBlueprintResources/StandardMacros.IncrementInt` _minutes))

(fn `CheckCondition`
  (params (Context :type "DlgContext Object Reference") (ConditionName :type Name))
  (returns (ReturnValue :type Boolean))
  (return false))

(fn `GetBoolValue`
  (params (ValueName :type Name))
  (returns (ReturnValue :type Boolean))
  (return false))

(fn `GetFloatValue`
  (params (ValueName :type Name))
  (returns (ReturnValue :type "Float (single-precision)"))
  (return 0.0))

(fn `GetIntValue`
  (params (ValueName :type Name))
  (returns (ReturnValue :type Integer))
  (return 0))

(fn `GetNameValue`
  (params (ValueName :type Name))
  (returns (ReturnValue :type Name))
  (return "None"))

(fn `GetParticipantDisplayName`
  (params (ActiveSpeaker :type Name))
  (returns (ReturnValue :type Text))
  (return (`self.Dlg_DisplayName`)))

(fn `GetParticipantGender`
  (returns (ReturnValue :type "ETextGender Enum"))
  (return "Masculine"))

(fn `GetParticipantIcon`
  (params (ActiveSpeaker :type Name) (ActiveSpeakerState :type Name))
  (returns (ReturnValue :type "Texture2D Object Reference"))
  (return "/Game/Deep-X-Pression/Assets/Clock.Clock"))

(fn `GetParticipantName`
  (returns (ReturnValue :type Name))
  (return (`self.Dlg_Name`)))

(fn `ModifyBoolValue`
  (params (ValueName :type Name) (bNewValue :type Boolean))
  (returns (ReturnValue :type Boolean))
  (return false))

(fn `ModifyFloatValue`
  (params (ValueName :type Name) (bDelta :type Boolean) (Value :type "Float (single-precision)"))
  (returns (ReturnValue :type Boolean))
  (return false))

(fn `ModifyIntValue`
  (params (ValueName :type Name) (bDelta :type Boolean) (Value :type Integer))
  (returns (ReturnValue :type Boolean))
  (return false))

(fn `ModifyNameValue`
  (params (ValueName :type Name) (NameValue :type Name))
  (returns (ReturnValue :type Boolean))
  (return false))

(fn `OnDialogueEvent`
  (params (Context :type "DlgContext Object Reference") (EventName :type Name))
  (returns (ReturnValue :type Boolean))
  (return false))

(fn `ResetFromDesk`
  (bind _otherclock (`self.OtherClock`))
  (bind _output_get (set `self.CanInteract` false))
  (set `/Game/Deep-X-Pression/Blueprints/BP_AnalogClock.CanInteract` _output_get _otherclock)
  (set `self.temp` (+ (`self.Minutes`) 1))
  (set `/Game/Deep-X-Pression/Blueprints/BP_AnalogClock.temp` (+ (`/Game/Deep-X-Pression/Blueprints/BP_AnalogClock.Minutes` _otherclock) 1) _otherclock))

(fn `SetDeskAdvance`
  (params (DeskAdvance :type Boolean))
  (bind _output_get (set `self.DeskAdvance` DeskAdvance))
  (set `/Game/Deep-X-Pression/Blueprints/BP_AnalogClock.DeskAdvance` _output_get (`self.OtherClock`)))

(fn `UserConstructionScript`)