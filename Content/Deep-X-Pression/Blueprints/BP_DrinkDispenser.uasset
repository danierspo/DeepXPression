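; Interactable drink dispenser that gives Emil a one-time effect and acts as a dialogue participant.
; Overlapping characters trigger a prompt widget and enable the Interact input until they leave.
; The first use sets Emil's Focus, applies a negative mood change, starts dialogue and locks both this and the paired OtherDispenser.
; Later presses only start the dialogue; the dialogue condition, value and event functions are default stubs.
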(event `self.ReceiveBeginPlay`
  ;[1 1 1] BeginPlay: obtain reference to BP_Emil player character
  (bind _asbp_emil (cast `/Game/Deep-X-Pression/Blueprints/BP_Emil` (`Controller.K2_GetPawn` (`GameplayStatics.GetPlayerController` 0))))
  (set `self.Emil` _asbp_emil))

(event `InputAction|Interact`
  (params (Key :type "Key Structure"))
  ;[1 1 1] Press E to interact with the dispenser
  (:`Pressed`
    (if (`self.CanInteract`)
      (`self.OnInteract`)
      (else
        (`/Game/Deep-X-Pression/Blueprints/BP_Emil.StartDialogue` (`self.Emil`) (`self.DialogueWithEmil`))))))

(event `self.ReceiveActorBeginOverlap`
  (params (OtherActor :type "Actor Object Reference"))
  ;[1 1 1] Dispenser overlapping with character
  (cast `Character` OtherActor)
  (bind _returnvalue (`|CreateWidget` "/Game/Deep-X-Pression/UI/InteractPrompts/IP_Dispenser.IP_Dispenser_C"))
  (`UserWidget.AddToViewport` _returnvalue 0)
  (`self.EnableInput` (`GameplayStatics.GetPlayerController` 0)))

(event `self.ReceiveActorEndOverlap`
  (params (OtherActor :type "Actor Object Reference"))
  ;[1 1 1] Dispenser overlapping with character
  (cast `Character` OtherActor)
  (`Widget.RemoveFromParent` (stale `self.ReceiveActorBeginOverlap` _returnvalue))
  (`self.DisableInput` (`GameplayStatics.GetPlayerController` 0)))

(event `self.OnInteract`
  (bind _emil (`self.Emil`))
  ;[1 1 1] Interactable's OnInteract method implementation
  (set `/Game/Deep-X-Pression/Blueprints/BP_Emil.Focus` true _emil)
  (`/Game/Deep-X-Pression/Blueprints/BP_Emil.AddToMood` _emil -25.0)
  (`/Game/Deep-X-Pression/Blueprints/BP_Emil.StartDialogue` _emil (`self.DialogueWithEmil`))
  (set `self.CanInteract` false)
  (set `/Game/Deep-X-Pression/Blueprints/BP_DrinkDispenser.CanInteract` false (`self.OtherDispenser`)))

(fn `CheckCondition`
  (params (Context :type "DlgContext Object Reference") (ConditionName :type Name))
  (returns (ReturnValue :type Boolean))
  (return false))

(fn `GetBoolValue`
  (params (ValueName :type Name))
  (returns (ReturnValue :type Boolean))
  (return false))

(fn `GetFloatValue`
  (params (ValueName :type Name))
  (returns (ReturnValue :type "Float (single-precision)"))
  (return 0.0))

(fn `GetIntValue`
  (params (ValueName :type Name))
  (returns (ReturnValue :type Integer))
  (return 0))

(fn `GetNameValue`
  (params (ValueName :type Name))
  (returns (ReturnValue :type Name))
  (return "None"))

(fn `GetParticipantDisplayName`
  (params (ActiveSpeaker :type Name))
  (returns (ReturnValue :type Text))
  (return (`self.DlgDisplayName`)))

(fn `GetParticipantGender`
  (returns (ReturnValue :type "ETextGender Enum"))
  (return "Masculine"))

(fn `GetParticipantIcon`
  (params (ActiveSpeaker :type Name) (ActiveSpeakerState :type Name))
  (returns (ReturnValue :type "Texture2D Object Reference"))
  (return (`self.DlgIcon`)))

(fn `GetParticipantName`
  (returns (ReturnValue :type Name))
  (return (`self.DlgName`)))

(fn `ModifyBoolValue`
  (params (ValueName :type Name) (bNewValue :type Boolean))
  (returns (ReturnValue :type Boolean))
  (return false))

(fn `ModifyFloatValue`
  (params (ValueName :type Name) (bDelta :type Boolean) (Value :type "Float (single-precision)"))
  (returns (ReturnValue :type Boolean))
  (return false))

(fn `ModifyIntValue`
  (params (ValueName :type Name) (bDelta :type Boolean) (Value :type Integer))
  (returns (ReturnValue :type Boolean))
  (return false))

(fn `ModifyNameValue`
  (params (ValueName :type Name) (NameValue :type Name))
  (returns (ReturnValue :type Boolean))
  (return false))

(fn `OnDialogueEvent`
  (params (Context :type "DlgContext Object Reference") (EventName :type Name))
  (returns (ReturnValue :type Boolean))
  (return false))

(fn `UserConstructionScript`)