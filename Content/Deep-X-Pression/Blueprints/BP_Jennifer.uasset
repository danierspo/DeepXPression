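; BP_Jennifer is an interactable NPC and dialogue participant that opens her conversation with the player, Emil, when CanInteract allows.
; DialogueEnd applies the mood change to Emil, clamps Relationship, closes conversation and updates WC's repeatable-dialogue state.
; Other functions suspend dialogue or flag work left on Emil's desk, while LoadData and SaveData persist Relationship in the Save1 slot.
; Dialogue interface methods supply her identity; condition, value and event handlers are stubs.
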(event `self.ReceiveBeginPlay`
  ;[1 1 1] BeginPlay: obtain reference to BP_Emil player character
  (bind _asbp_emil (cast `/Game/Deep-X-Pression/Blueprints/BP_Emil` (`Controller.K2_GetPawn` (`GameplayStatics.GetPlayerController` 0))))
  (set `self.Emil` _asbp_emil)
  (`self.LoadData`))

(event `/Game/Deep-X-Pression/Interfaces/Interactable.OnInteract`
  ;[1 1 1] Interactable's OnInteract method implementation
  (if (`self.CanInteract`)
    (`/Game/Deep-X-Pression/Blueprints/BP_Emil.StartDialogue` (`self.Emil`) "/Game/Deep-X-Pression/Dialogues/Dlg_EmilJennifer.Dlg_EmilJennifer")
    (else
      (`KismetSystemLibrary.PrintString` "Al momento non puoi interagire con Jennifer."))))

(fn `CheckCondition`
  (params (Context :type "DlgContext Object Reference") (ConditionName :type Name))
  (returns (ReturnValue :type Boolean))
  (return false))

(fn `DialogueEnd`
  (bind _relationship (`self.Relationship`))
  (`/Game/Deep-X-Pression/Blueprints/BP_Emil.AddToMood` (`self.Emil`) (`KismetMathLibrary.Conv_IntToDouble` (`self.MoodDifference`)))
  (if (> _relationship 100)
    (set `self.Relationship` 100)
    (elif (< _relationship 0)
      (set `self.Relationship` 0)))
  (set `self.CanConverse` false)
  (set `self.DialogueSuspended` false)
  (`/Game/Deep-X-Pression/Blueprints/BP_WC.SetRepeatableDialoguesJennifer` (`self.WC`) true))

(fn `GetBoolValue`
  (params (ValueName :type Name))
  (returns (ReturnValue :type Boolean))
  (return false))

(fn `GetFloatValue`
  (params (ValueName :type Name))
  (returns (ReturnValue :type "Float (single-precision)"))
  (return 0.0))

(fn `GetIntValue`
  (params (ValueName :type Name))
  (returns (ReturnValue :type Integer))
  (return 0))

(fn `GetNameValue`
  (params (ValueName :type Name))
  (returns (ReturnValue :type Name))
  (return "None"))

(fn `GetParticipantDisplayName`
  (params (ActiveSpeaker :type Name))
  (returns (ReturnValue :type Text))
  (return (`self.DisplayName`)))

(fn `GetParticipantGender`
  (returns (ReturnValue :type "ETextGender Enum"))
  (return "Masculine"))

(fn `GetParticipantIcon`
  (params (ActiveSpeaker :type Name) (ActiveSpeakerState :type Name))
  (returns (ReturnValue :type "Texture2D Object Reference"))
  (return "/Game/Deep-X-Pression/Assets/Jennifer.Jennifer"))

(fn `GetParticipantName`
  (returns (ReturnValue :type Name))
  (return "Jennifer"))

(fn `LeaveWorkToEmil`
  (set `self.WorkToDo` true)
  (set `/Game/Deep-X-Pression/Blueprints/BP_EmilDesk.WorkToDo_Jennifer` true (`self.EmilDesk`)))

(fn `LoadData`
  (bind _returnvalue (`GameplayStatics.DoesSaveGameExist` "Save1"))
  (if _returnvalue
    (bind _returnvalue_2 (`GameplayStatics.LoadGameFromSlot` "Save1"))
    (bind _asbp_save_game (cast `/Game/Deep-X-Pression/Other/BP_SaveGame` _returnvalue_2))
    (set `self.Relationship` (`/Game/Deep-X-Pression/Other/BP_SaveGame.Jennifer_Relationship` _asbp_save_game))
    (`KismetSystemLibrary.PrintString` "[Jennifer] GAME LOADED")
    (else
      (`KismetSystemLibrary.PrintString` "[Jennifer] PROBLEM: it should exist"))))

(fn `ModifyBoolValue`
  (params (ValueName :type Name) (bNewValue :type Boolean))
  (returns (ReturnValue :type Boolean))
  (return false))

(fn `ModifyFloatValue`
  (params (ValueName :type Name) (bDelta :type Boolean) (Value :type "Float (single-precision)"))
  (returns (ReturnValue :type Boolean))
  (return false))

(fn `ModifyIntValue`
  (params (ValueName :type Name) (bDelta :type Boolean) (Value :type Integer))
  (returns (ReturnValue :type Boolean))
  (return false))

(fn `ModifyNameValue`
  (params (ValueName :type Name) (NameValue :type Name))
  (returns (ReturnValue :type Boolean))
  (return false))

(fn `OnDialogueEvent`
  (params (Context :type "DlgContext Object Reference") (EventName :type Name))
  (returns (ReturnValue :type Boolean))
  (return false))

(fn `SaveData`
  (bind _bp_savegame (`/Game/Deep-X-Pression/Blueprints/BP_Emil.BP_SaveGame` (`self.Emil`)))
  (set `/Game/Deep-X-Pression/Other/BP_SaveGame.Jennifer_Relationship` (`self.Relationship`) _bp_savegame)
  (`GameplayStatics.SaveGameToSlot` _bp_savegame "Save1")
  (`KismetSystemLibrary.PrintString` "[Jennifer] GAME SAVED"))

(fn `SuspendDialogue`
  (set `self.DialogueSuspended` true)
  (`/Game/Deep-X-Pression/Blueprints/BP_Window.ToggleImportantDialogueJennifer` (`self.Window`)))

(fn `UserConstructionScript`)