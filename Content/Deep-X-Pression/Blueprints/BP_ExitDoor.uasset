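; Interactable exit door and dialogue participant through which Emil can end the workday.
; Overlapping characters see a prompt widget, and interacting starts one of Emil's dialogues depending on CanInteract.
; NextDay penalises Emil's mood and coworker relationships by time left until about 18:00 unless CanLeave, saves, fades out and reloads the level.
; GameOver fades out, shows a summary screen, deletes the save and pauses the game.
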(event `self.ReceiveBeginPlay`
  ;[1 1 1] BeginPlay: obtain reference to BP_Emil player character
  (bind _asbp_emil (cast `/Game/Deep-X-Pression/Blueprints/BP_Emil` (`Controller.K2_GetPawn` (`GameplayStatics.GetPlayerController` 0))))
  (set `self.Emil` _asbp_emil))

(event `InputAction|Interact`
  (params (Key :type "Key Structure"))
  ;[1 1 1] Press E to interact with the exit door
  (:`Pressed`
    (if (`self.CanInteract`)
      (`self.OnInteract`)
      (else
        (`/Game/Deep-X-Pression/Blueprints/BP_Emil.StartDialogue` (`self.Emil`) "/Game/Deep-X-Pression/Dialogues/Dlg_Emil_CannotInteract.Dlg_Emil_CannotInteract")))))

(event `self.ReceiveActorBeginOverlap`
  (params (OtherActor :type "Actor Object Reference"))
  ;[1 1 1] Dispenser overlapping with character
  (cast `Character` OtherActor)
  (bind _returnvalue (`|CreateWidget` "/Game/Deep-X-Pression/UI/InteractPrompts/IP_ExitDoor.IP_ExitDoor_C"))
  (`UserWidget.AddToViewport` _returnvalue 0)
  (`self.EnableInput` (`GameplayStatics.GetPlayerController` 0)))

(event `self.ReceiveActorEndOverlap`
  (params (OtherActor :type "Actor Object Reference"))
  ;[1 1 1] Dispenser overlapping with character
  (cast `Character` OtherActor)
  (`Widget.RemoveFromParent` (stale `self.ReceiveActorBeginOverlap` _returnvalue))
  (`self.DisableInput` (`GameplayStatics.GetPlayerController` 0)))

(event `self.OnInteract`
  ;[1 1 1] Interactable's OnInteract method implementation
  (`/Game/Deep-X-Pression/Blueprints/BP_Emil.StartDialogue` (`self.Emil`) "/Game/Deep-X-Pression/Dialogues/Dlg_EmilExitDoor.Dlg_EmilExitDoor"))

(event `GameOver`
  ;[1 1 1] Ends the game, showing a summarising screen (it's an event and not a function, because I wanted to implement a delay after the camera fade, and it's not callable inside a function)
  (`self.DisableInput` (`GameplayStatics.GetPlayerController` 0))
  (`PlayerCameraManager.StartCameraFade` (`GameplayStatics.GetPlayerCameraManager` 0) 0.0 1.0 1.0 (struct :`A` 1.0) true true)
  (`KismetSystemLibrary.Delay` 2.0)
  (bind _returnvalue (`|CreateWidget` "/Game/Deep-X-Pression/UI/WB_Summarising.WB_Summarising_C"))
  (`UserWidget.AddToViewport` _returnvalue 0)
  (`GameplayStatics.DeleteGameInSlot` "Save1")
  (`GameplayStatics.SetGamePaused` true))

(event `NextDay`
  (bind _kevin (`self.Kevin`))
  (bind _laura (`self.Laura`))
  (bind _emil (`self.Emil`))
  (bind _harry (`self.Harry`))
  ;[1 1 1] Goes to the next day, showing a summarising screen (it's an event and not a function, because I wanted to implement a delay after the camera fade, and it's not callable inside a function)
  (set `self.EndGame` false)
  (if (not (`self.CanLeave`))
    (bind _timepenalty (`self.ComputeTimePenalty`))
    (`/Game/Deep-X-Pression/Blueprints/BP_Emil.AddToMood` (`self.Emil`) (`KismetMathLibrary.Conv_IntToDouble` (`KismetMathLibrary.FTrunc` (* _timepenalty -1.0))))
    (bind _output_get (set `/Game/Deep-X-Pression/Other/BP_SecondaryCharacter.Relationship` (`KismetMathLibrary.FTrunc` (- (`/Game/Deep-X-Pression/Other/BP_SecondaryCharacter.Relationship` _harry) _timepenalty)) _harry))
    (if (< _output_get 0)
      (set `/Game/Deep-X-Pression/Other/BP_SecondaryCharacter.Relationship` 0 _harry))
    (bind _output_get_2 (set `/Game/Deep-X-Pression/Other/BP_SecondaryCharacter.Relationship` (`KismetMathLibrary.FTrunc` (- (`/Game/Deep-X-Pression/Other/BP_SecondaryCharacter.Relationship` _kevin) _timepenalty)) _kevin))
    (if (< _output_get_2 0)
      (set `/Game/Deep-X-Pression/Other/BP_SecondaryCharacter.Relationship` 0 _kevin))
    (bind _output_get_3 (set `/Game/Deep-X-Pression/Other/BP_SecondaryCharacter.Relationship` (`KismetMathLibrary.FTrunc` (- (`/Game/Deep-X-Pression/Other/BP_SecondaryCharacter.Relationship` _laura) _timepenalty)) _laura))
    (if (< _output_get_3 0)
      (set `/Game/Deep-X-Pression/Other/BP_SecondaryCharacter.Relationship` 0 _laura)))
  (`/Engine/EditorBlueprintResources/StandardMacros.IncrementInt` (`/Game/Deep-X-Pression/Blueprints/BP_Emil.Day` _emil)
    (:`  `
      (`/Game/Deep-X-Pression/Blueprints/BP_Emil.SaveData` _emil)
      (`/Game/Deep-X-Pression/Blueprints/BP_Harry.SaveData` (`self.Harry`))
      (`/Game/Deep-X-Pression/Blueprints/BP_Jennifer.SaveData` (`self.Jennifer`))
      (`/Game/Deep-X-Pression/Blueprints/BP_Kevin.SaveData` (`self.Kevin`))
      (`/Game/Deep-X-Pression/Blueprints/BP_Laura.SaveData` (`self.Laura`))
      (`PlayerCameraManager.StartCameraFade` (`GameplayStatics.GetPlayerCameraManager` 0) 0.0 1.0 1.0 (struct :`A` 1.0) true true)
      (`KismetSystemLibrary.Delay` 2.0)
      (`self.ResetLevel`))))

(fn `CheckCondition`
  (params (Context :type "DlgContext Object Reference") (ConditionName :type Name))
  (returns (ReturnValue :type Boolean))
  (return false))

(fn `ComputeTimePenalty`
  (returns (TimePenalty :type "Float (double-precision)"))
  (bind _clock (`self.Clock`))
  (bind _output_get (set `self.TimePenalty` (+ (* (- 17.0 (`KismetMathLibrary.Conv_IntToDouble` (`/Game/Deep-X-Pression/Blueprints/BP_AnalogClock.Hours` _clock))) 5.0) (/ (* (- 60.0 (`KismetMathLibrary.Conv_IntToDouble` (`/Game/Deep-X-Pression/Blueprints/BP_AnalogClock.Minutes` _clock))) 5.0) 60.0))))
  (return _output_get))

(fn `GetBoolValue`
  (params (ValueName :type Name))
  (returns (ReturnValue :type Boolean))
  (return false))

(fn `GetFloatValue`
  (params (ValueName :type Name))
  (returns (ReturnValue :type "Float (single-precision)"))
  (return 0.0))

(fn `GetIntValue`
  (params (ValueName :type Name))
  (returns (ReturnValue :type Integer))
  (return 0))

(fn `GetNameValue`
  (params (ValueName :type Name))
  (returns (ReturnValue :type Name))
  (return "None"))

(fn `GetParticipantDisplayName`
  (params (ActiveSpeaker :type Name))
  (returns (ReturnValue :type Text))
  (return (`self.DisplayName`)))

(fn `GetParticipantGender`
  (returns (ReturnValue :type "ETextGender Enum"))
  (return "Masculine"))

(fn `GetParticipantIcon`
  (params (ActiveSpeaker :type Name) (ActiveSpeakerState :type Name))
  (returns (ReturnValue :type "Texture2D Object Reference"))
  (return "/Game/Deep-X-Pression/Assets/ExitDoor.ExitDoor"))

(fn `GetParticipantName`
  (returns (ReturnValue :type Name))
  (return "ExitDoor"))

(fn `ModifyBoolValue`
  (params (ValueName :type Name) (bNewValue :type Boolean))
  (returns (ReturnValue :type Boolean))
  (return false))

(fn `ModifyFloatValue`
  (params (ValueName :type Name) (bDelta :type Boolean) (Value :type "Float (single-precision)"))
  (returns (ReturnValue :type Boolean))
  (return false))

(fn `ModifyIntValue`
  (params (ValueName :type Name) (bDelta :type Boolean) (Value :type Integer))
  (returns (ReturnValue :type Boolean))
  (return false))

(fn `ModifyNameValue`
  (params (ValueName :type Name) (NameValue :type Name))
  (returns (ReturnValue :type Boolean))
  (return false))

(fn `OnDialogueEvent`
  (params (Context :type "DlgContext Object Reference") (EventName :type Name))
  (returns (ReturnValue :type Boolean))
  (return false))

(fn `ResetLevel`
  (bind _returnvalue (`GameplayStatics.GetCurrentLevelName` true))
  (`GameplayStatics.OpenLevel` (`KismetStringLibrary.Conv_StringToName` _returnvalue)))

(fn `UserConstructionScript`)