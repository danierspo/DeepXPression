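; Interactable desk that lets the player character Emil sit down to work and stand up again.
; Overlap with a character shows a prompt widget and enables Interact input, which plays a dialogue line when interaction is disallowed.
; OnInteract toggles the seated state behind camera fades, switching movement, sitting montage and position.
; Sitting puts both linked clocks into desk-advance mode and locks their interaction; standing resets through the Clock reference.
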(event `self.ReceiveBeginPlay`
  ;[1 1 1] BeginPlay: obtain reference to BP_Emil player character
  (bind _asbp_emil (cast `/Game/Deep-X-Pression/Blueprints/BP_Emil` (`Controller.K2_GetPawn` (`GameplayStatics.GetPlayerController` 0))))
  (set `self.Emil` _asbp_emil))

(event `InputAction|Interact`
  (params (Key :type "Key Structure"))
  ;[1 1 1] Press E to interact with the desk
  (:`Pressed`
    (if (`self.CanInteract`)
      (`self.OnInteract`)
      (else
        (`/Game/Deep-X-Pression/Blueprints/BP_Emil.StartDialogue` (`self.Emil`) "/Game/Deep-X-Pression/Dialogues/Dlg_Emil_CannotInteract.Dlg_Emil_CannotInteract")))))

(event `self.ReceiveActorBeginOverlap`
  (params (OtherActor :type "Actor Object Reference"))
  ;[1 1 1] Desk overlapping with character
  (cast `Character` OtherActor)
  (bind _returnvalue (`|CreateWidget` "/Game/Deep-X-Pression/UI/InteractPrompts/IP_EmilDesk.IP_EmilDesk_C"))
  (`UserWidget.AddToViewport` _returnvalue 0)
  (`self.EnableInput` (`GameplayStatics.GetPlayerController` 0)))

(event `self.ReceiveActorEndOverlap`
  (params (OtherActor :type "Actor Object Reference"))
  ;[1 1 1] Desk overlapping with character
  (cast `Character` OtherActor)
  (`Widget.RemoveFromParent` (stale `self.ReceiveActorBeginOverlap` _returnvalue))
  (`self.DisableInput` (`GameplayStatics.GetPlayerController` 0)))

(event `self.OnInteract`
  (bind (_returnvalue_roll _returnvalue_pitch _returnvalue_yaw) (`KismetMathLibrary.BreakRotator` (`self.K2_GetActorRotation`)))
  (bind (_returnvalue_roll_2 _returnvalue_pitch_2 _returnvalue_yaw_2) (`KismetMathLibrary.BreakRotator` (`self.K2_GetActorRotation`)))
  (bind _returnvalue (`GameplayStatics.GetPlayerCameraManager` 0))
  (bind _returnvalue_2 (`GameplayStatics.GetPlayerCameraManager` 0))
  (bind _emil (`self.Emil`))
  (bind _emil_2 (`self.Emil`))
  (bind _clock (`self.Clock`))
  (bind _clock_2 (`self.Clock`))
  (bind _otherclock (`/Game/Deep-X-Pression/Blueprints/BP_AnalogClock.OtherClock` _clock))
  ;[1 1 1] Interactable's OnInteract method implementation
  (if (not (`self.Working`))
    (`PlayerCameraManager.StartCameraFade` _returnvalue_2 0.0 1.0 1.0 (struct :`A` 1.0) false true)
    (`KismetSystemLibrary.Delay` 1.0)
    (`ActorComponent.ToggleActive` (`Character.CharacterMovement` _emil_2))
    (`Character.PlayAnimMontage` _emil_2 "/Game/Deep-X-Pression/Animations/Male_Sitting_Pose_Montage.Male_Sitting_Pose_Montage" 1.0 "None")
    (`KismetSystemLibrary.MoveComponentTo` (`Actor.RootComponent` _emil_2) (+ (`self.K2_GetActorLocation`) (`KismetMathLibrary.MakeVector` 0.0 -97.5 (`CapsuleComponent.CapsuleHalfHeight` (`Character.CapsuleComponent` _emil_2)))) (`KismetMathLibrary.MakeRotator` 0.0 0.0 (+ _returnvalue_yaw_2 90.0)) true true 0.5 true)
    (`KismetSystemLibrary.Delay` 1.0)
    (`PlayerCameraManager.StartCameraFade` _returnvalue_2 1.0 0.0 1.0 (struct :`A` 1.0) false true)
    (set `/Game/Deep-X-Pression/Blueprints/BP_AnalogClock.DeskAdvance` true _clock)
    (set `/Game/Deep-X-Pression/Blueprints/BP_AnalogClock.CanInteract` false _clock)
    (set `/Game/Deep-X-Pression/Blueprints/BP_AnalogClock.DeskAdvance` true _otherclock)
    (set `/Game/Deep-X-Pression/Blueprints/BP_AnalogClock.CanInteract` false _otherclock)
    (set `self.Working` true)
    (else
      (`PlayerCameraManager.StartCameraFade` _returnvalue 0.0 1.0 1.0 (struct :`A` 1.0) false true)
      (`KismetSystemLibrary.Delay` 1.0)
      (`ActorComponent.ToggleActive` (`Character.CharacterMovement` _emil))
      (`Character.StopAnimMontage` _emil "/Game/Deep-X-Pression/Animations/Male_Sitting_Pose_Montage.Male_Sitting_Pose_Montage")
      (`KismetSystemLibrary.MoveComponentTo` (`Actor.RootComponent` _emil) (+ (`self.K2_GetActorLocation`) (`KismetMathLibrary.MakeVector` 200.0 -50.0 (`CapsuleComponent.CapsuleHalfHeight` (`Character.CapsuleComponent` _emil)))) (`KismetMathLibrary.MakeRotator` 0.0 0.0 (+ _returnvalue_yaw 90.0)) true true 0.5 true)
      (`KismetSystemLibrary.Delay` 1.0)
      (`PlayerCameraManager.StartCameraFade` _returnvalue 1.0 0.0 1.0 (struct :`A` 1.0) false true)
      (set `self.Working` false)
      (`/Game/Deep-X-Pression/Blueprints/BP_AnalogClock.SetDeskAdvance` _clock_2 false)
      (`/Game/Deep-X-Pression/Blueprints/BP_AnalogClock.ResetFromDesk` _clock_2))))

(fn `UserConstructionScript`)