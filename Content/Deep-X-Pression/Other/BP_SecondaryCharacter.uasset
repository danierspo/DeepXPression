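; Base-style secondary character actor that the player interacts with on the Interact input while nearby.
; Overlap with any Character shows an IP_SecondaryCharacter widget and enables input, and ending the overlap removes both.
; Interact calls OnInteract when CanInteract is set, otherwise Emil starts a cannot-interact dialogue.
; RestoreRelationship subtracts MoodDifference from the Relationship value.
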(event `InputAction|Interact`
  (params (Key :type "Key Structure"))
  ;[1 1 1] Press E to interact with the secondary character
  (:`Pressed`
    (if (`self.CanInteract`)
      (`self.OnInteract`)
      (else
        (`/Game/Deep-X-Pression/Blueprints/BP_Emil.StartDialogue` (`self.Emil`) "/Game/Deep-X-Pression/Dialogues/Dlg_Emil_CannotInteract.Dlg_Emil_CannotInteract")))))

(event `self.ReceiveActorBeginOverlap`
  (params (OtherActor :type "Actor Object Reference"))
  ;[1 1 1] Secondary character overlapping with player character
  (cast `Character` OtherActor)
  (bind _returnvalue (`|CreateWidget` "/Game/Deep-X-Pression/UI/InteractPrompts/IP_SecondaryCharacter.IP_SecondaryCharacter_C"))
  (`UserWidget.AddToViewport` _returnvalue 0)
  (`self.EnableInput` (`GameplayStatics.GetPlayerController` 0)))

(event `self.ReceiveActorEndOverlap`
  (params (OtherActor :type "Actor Object Reference"))
  ;[1 1 1] Secondary character overlapping with player character
  (cast `Character` OtherActor)
  (`Widget.RemoveFromParent` (stale `self.ReceiveActorBeginOverlap` _returnvalue))
  (`self.DisableInput` (`GameplayStatics.GetPlayerController` 0)))

(fn `RestoreRelationship`
  (set `self.Relationship` (- (`self.Relationship`) (`self.MoodDifference`))))

(fn `UserConstructionScript`)