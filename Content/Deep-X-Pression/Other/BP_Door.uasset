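; BP_Door is an interactable door that the player opens and closes with the Interact input.
; Character overlap shows an IP_Door widget and enables input on the actor for player 0, and leaving removes both.
; Interact calls OnInteract, the Interactable implementation, which uses a Closed flag to snap the mesh between a fixed open rotation and DefaultZRotation yaw, without animation.
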(event `InputAction|Interact`
  (params (Key :type "Key Structure"))
  ;[1 1 1] Press E to open the door
  (:`Pressed`
    (`self.OnInteract`)))

(event `self.ReceiveActorBeginOverlap`
  (params (OtherActor :type "Actor Object Reference"))
  ;[1 1 1] Door overlapping with character
  (cast `Character` OtherActor)
  (bind _returnvalue (`|CreateWidget` "/Game/Deep-X-Pression/UI/InteractPrompts/IP_Door.IP_Door_C"))
  (`UserWidget.AddToViewport` _returnvalue 0)
  (`self.EnableInput` (`GameplayStatics.GetPlayerController` 0)))

(event `self.ReceiveActorEndOverlap`
  (params (OtherActor :type "Actor Object Reference"))
  ;[1 1 1] Door overlapping with character
  (cast `Character` OtherActor)
  (`Widget.RemoveFromParent` (stale `self.ReceiveActorBeginOverlap` _returnvalue))
  (`self.DisableInput` (`GameplayStatics.GetPlayerController` 0)))

(event `self.OnInteract`
  (bind _staticmeshcomponent (`self.StaticMeshComponent`))
  ;[1 1 1] Interactable's OnInteract method implementation
  (if (`self.Closed`)
    (`SceneComponent.K2_SetRelativeRotation` _staticmeshcomponent (struct :`Yaw` 180.0) false false)
    (set `self.Closed` false)
    (else
      (`SceneComponent.K2_SetRelativeRotation` _staticmeshcomponent (`KismetMathLibrary.MakeRotator` 0.0 0.0 (`self.DefaultZRotation`)) false false)
      (set `self.Closed` true))))

(fn `UserConstructionScript`)